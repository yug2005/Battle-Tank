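; Tank Blueprint that wires player input to the tank's movement, aiming, firing and camera.
; BeginPlay initializes TankAiming with the barrel and turret, and TankMovement with the left and right tracks.
; Both movement axis events share one MoveTank call, while Fire calls TankAiming.
; Aim axes rotate separate horizontal and vertical gimbals in local space, keeping camera yaw and pitch independent.
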(event EventBeginPlay
  (Class|TankAimingComponent|Initialize (Variables|Default|GetTank%20Aiming) (Variables|Default|GetTank%20Barrel) (Variables|Default|GetTank%20Turret))
  (Class|TankMovementComponent|Initialize (Variables|Default|GetTank%20Movement) (Variables|Default|GetTank%20Left%20Track) (Variables|Default|GetTank%20Right%20Track)))

(event Input|ActionEvents|InputActionFire
  (params (Key :type Key%20Structure))
  ;[1 1 1] Aiming Input Binding
  (:Pressed
    (Class|TankAimingComponent|Fire (Variables|Default|GetTank%20Aiming))))

(event Input|ActionEvents|InputActionAim
  (params (Key :type Key%20Structure))
  ;[1 1 1] Aiming Input Binding
)

(event Input|AxisEvents|InputAxisAimHorizontal
  (params (AxisValue :type Float%20%28single-precision%29))
  ;[1 1 1] Camera Input Binding
  (Transformation|AddLocalRotation (Variables|Default|GetTank%20Horizontal%20Gimbal) (Math|Rotator|MakeRotator 0.0 0.0 AxisValue) false false))

(event Input|AxisEvents|InputAxisAimVertical
  (params (AxisValue :type Float%20%28single-precision%29))
  ;[1 1 1] Camera Input Binding
  (Transformation|AddLocalRotation (Variables|Default|GetTank%20Vertical%20Gimbal) (Math|Rotator|MakeRotator 0.0 AxisValue 0.0) false false))

(event Input|AxisEvents|InputAxisMovementX-Axis
  (params (AxisValue :type Float%20%28single-precision%29))
  ;[1 1 1] Movement Input Binding
  (Class|TankMovementComponent|MoveTank (Variables|Default|GetTank%20Movement) AxisValue (stale Input|AxisEvents|InputAxisMovementY-Axis AxisValue)))

(event Input|AxisEvents|InputAxisMovementY-Axis
  (params (AxisValue :type Float%20%28single-precision%29))
  ;[1 1 1] Movement Input Binding
  (Class|TankMovementComponent|MoveTank (Variables|Default|GetTank%20Movement) (stale Input|AxisEvents|InputAxisMovementX-Axis AxisValue) AxisValue))

(fn ConstructionScript)